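; BP_Collectable is a pickup actor that passes its mesh to the first-person player character when collected.
; On BeginPlay, a timeline animates the Shiner intensity by multiplying its current value by the track each update, so changes compound.
; The Collect event copies the Cube component's mesh onto player 0's StaticMesh component, then destroys the actor.
; Overlap and Tick are unused, and nothing here calls Collect.
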(event EventBeginPlay
  (bind _shiner (Variables|Default|Getshiner))
  (bind _newtrack_0 (Timeline|Timeline Play)
    (:Update
      (Rendering|Components|Light|SetIntensity _shiner (* (Variables|/Script/Engine.LightComponentBase|GetIntensity _shiner) _newtrack_0)))))

(event Collision|EventActorBeginOverlap
  (params (OtherActor :type Actor%20Object%20Reference)))

(event EventTick
  (params (DeltaSeconds :type Float%20%28single-precision%29)))

(event EventCollect
  (bind _asbp_first_person_character (Utilities|Casting|CastToBP_FirstPersonCharacter (Game|GetPlayerCharacter 0)))
  (Components|StaticMesh|SetStaticMesh (Variables|/Game/FirstPerson/Blueprints/BP_FirstPersonCharacter.BP_FirstPersonCharacter_C|GetStaticMesh _asbp_first_person_character) (Variables|/Script/Engine.StaticMeshComponent|GetStaticMesh (Variables|Default|GetCube)))
  (Actor|DestroyActor))

(fn ConstructionScript)